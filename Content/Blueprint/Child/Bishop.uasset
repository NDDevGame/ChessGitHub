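; Bishop chess piece, a child Blueprint that sets its ID on BeginPlay and highlights its diagonal moves.
; Move converts the given location to grid indices, then four bounded loops step X and Y together along each diagonal.
; Candidate squares are scaled to 400-unit world coordinates in Vecto2D and passed to the chessboard's ShowWayMove.
; The loops check only board-edge limits, with no test for occupied squares.
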(event EventBeginPlay
  (|CallParentFunction)
  (Variables|Default|SetID (Variables|Default|GetBishopName)))

(event Collision|EventActorBeginOverlap
  (params (OtherActor :type Actor%20Object%20Reference))
  (|CallParentFunction OtherActor) ; This node is disabled and will not be called.\nDrag off pins to build functionality.
)

(event EventTick
  (params (DeltaSeconds :type Float%20%28single-precision%29))
  (|CallParentFunction DeltaSeconds) ; This node is disabled and will not be called.\nDrag off pins to build functionality.
)

(event EventMove
  (params (Location :type Vector :default "0, 0, 0") (ChessBoard :type Chess%20Board%20Object%20Reference))
  (Utilities|Array|Clear (Variables|Default|GetVecto2D))
  (CallFunction|SetPositiontoXYValue Location)
  (Utilities|FlowControl|Sequence
    (:then_0
      ;[1 1 1] Move 45 degree
      (Variables|Default|SetTempNextYIndex (Math|Float|Floor (Variables|Default|GetYvalue)))
      (Variables|Default|SetTempNextXIndex (Math|Float|Floor (Variables|Default|GetXvalue)))
      (for _index (range 0 7) ; X Movement
        (if (and (<= (Variables|Default|GetTempNextXIndex) 7) (>= (Variables|Default|GetTempNextXIndex) 0))
          (bind _result (Math|Integer|IncrementInt (Variables|Default|GetTempNextXIndex))
            (:%20%20
              (bind _result_2 (Math|Integer|IncrementInt (Variables|Default|GetTempNextYIndex))
                (:%20%20
                  (Utilities|Array|Add (Variables|Default|GetVecto2D) (Math|Vector2D|MakeVector2D (* (Math|Conversions|ToFloat(Integer) _result) 4e+02) (* (Math|Conversions|ToFloat(Integer) _result_2) 4e+02)))))))))
      (Variables|Default|SetTempNextXIndex (Math|Float|Floor (Variables|Default|GetXvalue)))
      (Variables|Default|SetTempNextYIndex (Math|Float|Floor (Variables|Default|GetYvalue)))
      (for _index_2 (range 0 7) ; Y Movement
        (if (Math|Boolean|ANDBoolean (>= (Variables|Default|GetTempNextYIndex) 0) (!= (Variables|Default|GetTempNextXIndex) 7) (<= (Variables|Default|GetTempNextYIndex) 7))
          (Math|Integer|DecrementInt (Variables|Default|GetTempNextYIndex)
            (:%20%20
              (Math|Integer|IncrementInt (Variables|Default|GetTempNextXIndex)
                (:%20%20
                  (Utilities|Array|Add (Variables|Default|GetVecto2D) (Math|Vector2D|MakeVector2D (* (Math|Conversions|ToFloat(Integer) (Variables|Default|GetTempNextXIndex)) 4e+02) (* (Math|Conversions|ToFloat(Integer) (Variables|Default|GetTempNextYIndex)) 4e+02))))))))))
    (:then_1
      ;[1 1 1] move 45 degree left
      (Variables|Default|SetTempNextYIndex (Math|Float|Floor (Variables|Default|GetYvalue)))
      (Variables|Default|SetTempNextXIndex (Math|Float|Floor (Variables|Default|GetXvalue)))
      (for _index_3 (range 0 7) ; X Movement
        (if (Math|Boolean|ANDBoolean (<= (Variables|Default|GetTempNextXIndex) 7) (>= (Variables|Default|GetTempNextXIndex) 0) (!= (Variables|Default|GetTempNextYIndex) 0))
          (bind _result_3 (Math|Integer|DecrementInt (Variables|Default|GetTempNextYIndex))
            (:%20%20
              (bind _result_4 (Math|Integer|DecrementInt (Variables|Default|GetTempNextXIndex))
                (:%20%20
                  (Utilities|Array|Add (Variables|Default|GetVecto2D) (Math|Vector2D|MakeVector2D (* (Math|Conversions|ToFloat(Integer) _result_4) 4e+02) (* (Math|Conversions|ToFloat(Integer) _result_3) 4e+02)))))))))
      (Variables|Default|SetTempNextXIndex (Math|Float|Floor (Variables|Default|GetXvalue)))
      (Variables|Default|SetTempNextYIndex (Math|Float|Floor (Variables|Default|GetYvalue)))
      (for _index_4 (range 0 7) ; Y Movement
        (if (Math|Boolean|ANDBoolean (>= (Variables|Default|GetTempNextYIndex) 0) (<= (Variables|Default|GetTempNextYIndex) 7) true)
          (bind _result_5 (Math|Integer|IncrementInt (Variables|Default|GetTempNextYIndex))
            (:%20%20
              (bind _result_6 (Math|Integer|DecrementInt (Variables|Default|GetTempNextXIndex))
                (:%20%20
                  (Utilities|Array|Add (Variables|Default|GetVecto2D) (Math|Vector2D|MakeVector2D (* (Math|Conversions|ToFloat(Integer) _result_6) 4e+02) (* (Math|Conversions|ToFloat(Integer) _result_5) 4e+02)))))))))))
  (Variables|Default|SetTempNextXIndex (Math|Float|Floor (Variables|Default|GetXvalue)))
  (Variables|Default|SetTempNextYIndex (Math|Float|Floor (Variables|Default|GetYvalue)))
  (Default|ShowWayMove ChessBoard (Variables|Default|GetVecto2D)))

(fn ConstructionScript
  (|CallParentFunction))