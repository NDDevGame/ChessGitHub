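; Pawn chess piece that works out its candidate forward and diagonal-capture squares for display on the board.
; Move branches on side and first move to step one or two squares along X and probe both forward diagonals on a 400-unit grid.
; Line-trace macros test occupancy and piece side, filling Vecto2D for ChessBoard.ShowWayMove.
; An index-based PawnMovement function holds only disconnected logic.
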(event EventBeginPlay
  (|CallParentFunction)
  (Variables|Default|SetID (Variables|Default|GetPawnName)))

(event Collision|EventActorBeginOverlap
  (params (OtherActor :type Actor%20Object%20Reference))
  (|CallParentFunction OtherActor) ; This node is disabled and will not be called.\nDrag off pins to build functionality.
)

(event EventTick
  (params (DeltaSeconds :type Float%20%28single-precision%29))
  (|CallParentFunction DeltaSeconds) ; This node is disabled and will not be called.\nDrag off pins to build functionality.
)

(event EventMove
  (params (Location :type Vector :default "0, 0, 0") (ChessBoard :type Chess%20Board%20Object%20Reference))
  (Utilities|Array|Clear (Variables|Default|GetVecto2D))
  (CallFunction|SetPositiontoXYValue Location)
  (if (Variables|Default|GetFirstMove)
    (if (Variables|Default|GetSide)
      (Utilities|FlowControl|Sequence
        (:then_0
          ;[0 1 0.9727] Black first Step
          (Variables|Default|SetTempNextXIndex (Math|Float|Floor (Variables|Default|GetXvalue)))
          (Utilities|FlowControl|ForLoopwithBreak 0 1 :!label _label
            (:LoopBody
              (if (and (<= (Variables|Default|GetTempNextXIndex) 7) (>= (Variables|Default|GetTempNextXIndex) 0))
                (bind _output_get (Variables|Default|SetTempNextXIndex (- (Variables|Default|GetTempNextXIndex) 1)))
                (Utilities|CheckforValidity (Math|Vector2D|MakeVector2D (* (Math|Conversions|ToFloat(Integer) _output_get) 4e+02) (* (Variables|Default|GetYvalue) 4e+02))
                  (:True
                    (goto _label Break)))))
            (:Completed
              (Variables|Default|SetTempNextXIndex (Math|Float|Floor (Variables|Default|GetXvalue)))
              (Default|ShowWayMove ChessBoard (Variables|Default|GetVecto2D) :!label _label_2))))
        (:then_1
          ;[1 0.4332 0] Rid of  one White pieces
          (Utilities|FlowControl|Sequence :!label _label_3
            (:then_0
              (Variables|Default|SetTempNextYIndex (Math|Float|Floor (Variables|Default|GetYvalue)))
              (Variables|Default|SetTempNextXIndex (Math|Float|Floor (Variables|Default|GetXvalue)))
              (if (and (<= (Variables|Default|GetTempNextXIndex) 7) (>= (Variables|Default|GetTempNextXIndex) 0))
                (bind _output_get_2 (Variables|Default|SetTempNextXIndex (- (Variables|Default|GetTempNextXIndex) 1)))
                (bind _output_get_3 (Variables|Default|SetTempNextYIndex (+ (Variables|Default|GetTempNextYIndex) 1)))
                (Utilities|CheckforValidityOtherSide (Math|Vector2D|MakeVector2D (* (Math|Conversions|ToFloat(Integer) _output_get_2) 4e+02) (* (Math|Conversions|ToFloat(Integer) _output_get_3) 4e+02))
                  (:True
                    (Variables|Default|SetTempNextXIndex (Math|Float|Floor (Variables|Default|GetXvalue)))
                    (Variables|Default|SetTempNextYIndex (Math|Float|Floor (Variables|Default|GetYvalue)))
                    (goto _label_2)))))
            (:then_1
              (Variables|Default|SetTempNextYIndex (Math|Float|Floor (Variables|Default|GetYvalue)))
              (Variables|Default|SetTempNextXIndex (Math|Float|Floor (Variables|Default|GetXvalue)))
              (if (and (<= (Variables|Default|GetTempNextXIndex) 7) (>= (Variables|Default|GetTempNextXIndex) 0))
                (bind _output_get_4 (Variables|Default|SetTempNextXIndex (- (Variables|Default|GetTempNextXIndex) 1)))
                (bind _output_get_5 (Variables|Default|SetTempNextYIndex (- (Variables|Default|GetTempNextYIndex) 1)))
                (Utilities|CheckforValidityOtherSide (Math|Vector2D|MakeVector2D (* (Math|Conversions|ToFloat(Integer) _output_get_4) 4e+02) (* (Math|Conversions|ToFloat(Integer) _output_get_5) 4e+02))
                  (:True
                    (Variables|Default|SetTempNextXIndex (Math|Float|Floor (Variables|Default|GetXvalue)))
                    (Variables|Default|SetTempNextYIndex (Math|Float|Floor (Variables|Default|GetYvalue)))
                    (goto _label_2))))))))
      (else
        (Utilities|FlowControl|Sequence
          (:then_0
            ;[1 0.3869 0.4869] White Frist Step
            (Variables|Default|SetTempNextXIndex (Math|Float|Floor (Variables|Default|GetXvalue)))
            (Utilities|FlowControl|ForLoopwithBreak 0 1 :!label _label_4
              (:LoopBody
                (if (and (<= (Variables|Default|GetTempNextXIndex) 7) (>= (Variables|Default|GetTempNextXIndex) 0))
                  (bind _output_get_6 (Variables|Default|SetTempNextXIndex (+ (Variables|Default|GetTempNextXIndex) 1)))
                  (Utilities|CheckforValidity (Math|Vector2D|MakeVector2D (* (Math|Conversions|ToFloat(Integer) _output_get_6) 4e+02) (* (Variables|Default|GetYvalue) 4e+02))
                    (:True
                      (goto _label_4 Break)))))
              (:Completed
                (Variables|Default|SetTempNextXIndex (Math|Float|Floor (Variables|Default|GetXvalue)))
                (goto _label_2))))
          (:then_1
            ;[0.9759 0.2684 1] Rid of one blackpiece
            (Utilities|FlowControl|Sequence :!label _label_5
              (:then_0
                (Variables|Default|SetTempNextYIndex (Math|Float|Floor (Variables|Default|GetYvalue)))
                (Variables|Default|SetTempNextXIndex (Math|Float|Floor (Variables|Default|GetXvalue)))
                (if (and (<= (Variables|Default|GetTempNextXIndex) 7) (>= (Variables|Default|GetTempNextXIndex) 0))
                  (bind _output_get_7 (Variables|Default|SetTempNextXIndex (+ (Variables|Default|GetTempNextXIndex) 1)))
                  (bind _output_get_8 (Variables|Default|SetTempNextYIndex (+ (Variables|Default|GetTempNextYIndex) 1)))
                  (Utilities|CheckforValidityOtherSide (Math|Vector2D|MakeVector2D (* (Math|Conversions|ToFloat(Integer) _output_get_7) 4e+02) (* (Math|Conversions|ToFloat(Integer) _output_get_8) 4e+02))
                    (:True
                      (Variables|Default|SetTempNextXIndex (Math|Float|Floor (Variables|Default|GetXvalue)))
                      (Variables|Default|SetTempNextYIndex (Math|Float|Floor (Variables|Default|GetYvalue)))
                      (goto _label_2)))))
              (:then_1
                (Variables|Default|SetTempNextYIndex (Math|Float|Floor (Variables|Default|GetYvalue)))
                (Variables|Default|SetTempNextXIndex (Math|Float|Floor (Variables|Default|GetXvalue)))
                (if (and (<= (Variables|Default|GetTempNextXIndex) 7) (>= (Variables|Default|GetTempNextXIndex) 0))
                  (bind _output_get_9 (Variables|Default|SetTempNextXIndex (+ (Variables|Default|GetTempNextXIndex) 1)))
                  (bind _output_get_10 (Variables|Default|SetTempNextYIndex (- (Variables|Default|GetTempNextYIndex) 1)))
                  (Utilities|CheckforValidityOtherSide (Math|Vector2D|MakeVector2D (* (Math|Conversions|ToFloat(Integer) _output_get_9) 4e+02) (* (Math|Conversions|ToFloat(Integer) _output_get_10) 4e+02))
                    (:True
                      (Variables|Default|SetTempNextXIndex (Math|Float|Floor (Variables|Default|GetXvalue)))
                      (Variables|Default|SetTempNextYIndex (Math|Float|Floor (Variables|Default|GetYvalue)))
                      (goto _label_2))))))))))
    (elif (Variables|Default|GetSide)
      (Utilities|FlowControl|Sequence
        (:then_0
          ;[0 1 0.0357] Black Move
          (Variables|Default|SetTempNextXIndex (Math|Float|Floor (Variables|Default|GetXvalue)))
          (if (and (<= (Variables|Default|GetTempNextXIndex) 7) (>= (Variables|Default|GetTempNextXIndex) 0))
            (bind _output_get_11 (Variables|Default|SetTempNextXIndex (- (Variables|Default|GetTempNextXIndex) 1)))
            (Utilities|CheckforValidity (Math|Vector2D|MakeVector2D (* (Math|Conversions|ToFloat(Integer) _output_get_11) 4e+02) (* (Variables|Default|GetYvalue) 4e+02))
              (:True
                _)
              (:False
                _))
            (Variables|Default|SetTempNextXIndex (Math|Float|Floor (Variables|Default|GetXvalue)))
            (goto _label_2)))
        (:then_1
          (goto _label_3)))
      (else
        (Utilities|FlowControl|Sequence
          (:then_0
            ;[0.07099 0.07567 1] White Move
            (Variables|Default|SetTempNextXIndex (Math|Float|Floor (Variables|Default|GetXvalue)))
            (if (and (<= (Variables|Default|GetTempNextXIndex) 7) (>= (Variables|Default|GetTempNextXIndex) 0))
              (bind _output_get_12 (Variables|Default|SetTempNextXIndex (+ (Variables|Default|GetTempNextXIndex) 1)))
              (Utilities|CheckforValidity (Math|Vector2D|MakeVector2D (* (Math|Conversions|ToFloat(Integer) _output_get_12) 4e+02) (* (Variables|Default|GetYvalue) 4e+02))
                (:True
                  _)
                (:False
                  _))
              (Variables|Default|SetTempNextXIndex (Math|Float|Floor (Variables|Default|GetXvalue)))
              (goto _label_2)))
          (:then_1
            (goto _label_5)))))))

(fn ConstructionScript
  (|CallParentFunction))

(fn PawnMovement
  (params (Index :type Integer)))