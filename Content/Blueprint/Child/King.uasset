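; King is a child Blueprint for a King, likely a board game piece, that builds on a parent class.
; On BeginPlay it runs the parent logic, then sets its ID to KingName.
; Its Move event only clears the Vecto2D collection and computes no moves.
; Construction defers to the parent, and the overlap and Tick events are disabled stubs.
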(event EventBeginPlay
  (|CallParentFunction)
  (Variables|Default|SetID (Variables|Default|GetKingName)))

(event Collision|EventActorBeginOverlap
  (params (OtherActor :type Actor%20Object%20Reference))
  (|CallParentFunction OtherActor) ; This node is disabled and will not be called.\nDrag off pins to build functionality.
)

(event EventTick
  (params (DeltaSeconds :type Float%20%28single-precision%29))
  (|CallParentFunction DeltaSeconds) ; This node is disabled and will not be called.\nDrag off pins to build functionality.
)

(event EventMove
  (params (Location :type Vector :default "0, 0, 0") (ChessBoard :type Chess%20Board%20Object%20Reference))
  (Utilities|Array|Clear (Variables|Default|GetVecto2D)))

(fn ConstructionScript
  (|CallParentFunction))