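; Knight chess piece Blueprint that sets its ID on BeginPlay and computes the knight's candidate moves.
; Move converts the given location to grid indices, then a Sequence adds the eight L-shaped offsets, scaled to 400-unit squares, to Vecto2D.
; The growing array goes to ChessBoard.ShowWayMove after each addition.
; The range check tests only the starting X, so off-board targets are not filtered here.
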(event EventBeginPlay
  (|CallParentFunction)
  (Variables|Default|SetID (Variables|Default|GetKnightName)))

(event Collision|EventActorBeginOverlap
  (params (OtherActor :type Actor%20Object%20Reference))
  (|CallParentFunction OtherActor) ; This node is disabled and will not be called.\nDrag off pins to build functionality.
)

(event EventTick
  (params (DeltaSeconds :type Float%20%28single-precision%29))
  (|CallParentFunction DeltaSeconds) ; This node is disabled and will not be called.\nDrag off pins to build functionality.
)

(event EventMove
  (params (Location :type Vector :default "0, 0, 0") (ChessBoard :type Chess%20Board%20Object%20Reference))
  (Utilities|Array|Clear (Variables|Default|GetVecto2D))
  (CallFunction|SetPositiontoXYValue Location)
  (Utilities|FlowControl|Sequence
    (:then_0
      ;[1 1 1] x+1, y - 2
      (Variables|Default|SetTempNextYIndex (Math|Float|Floor (Variables|Default|GetYvalue)))
      (Variables|Default|SetTempNextXIndex (Math|Float|Floor (Variables|Default|GetXvalue)))
      (if (and (<= (Variables|Default|GetTempNextXIndex) 7) (>= (Variables|Default|GetTempNextXIndex) 0))
        (bind _result (Math|Integer|IncrementInt (Variables|Default|GetTempNextXIndex))
          (:%20%20
            (bind _output_get (Variables|Default|SetTempNextYIndex (- (Variables|Default|GetTempNextYIndex) 2)))
            (Utilities|Array|Add (Variables|Default|GetVecto2D) (Math|Vector2D|MakeVector2D (* (Math|Conversions|ToFloat(Integer) _result) 4e+02) (* (Math|Conversions|ToFloat(Integer) _output_get) 4e+02)))
            (Default|ShowWayMove ChessBoard (Variables|Default|GetVecto2D) :!label _label)))))
    (:then_1
      ;[1 1 1] x+2,y-1
      (Variables|Default|SetTempNextYIndex (Math|Float|Floor (Variables|Default|GetYvalue)))
      (Variables|Default|SetTempNextXIndex (Math|Float|Floor (Variables|Default|GetXvalue)))
      (if (and (<= (Variables|Default|GetTempNextXIndex) 7) (>= (Variables|Default|GetTempNextXIndex) 0))
        (bind _output_get_2 (Variables|Default|SetTempNextXIndex (+ (Variables|Default|GetTempNextXIndex) 2)))
        (bind _output_get_3 (Variables|Default|SetTempNextYIndex (- (Variables|Default|GetTempNextYIndex) 1)))
        (Utilities|Array|Add (Variables|Default|GetVecto2D) (Math|Vector2D|MakeVector2D (* (Math|Conversions|ToFloat(Integer) _output_get_2) 4e+02) (* (Math|Conversions|ToFloat(Integer) _output_get_3) 4e+02)))
        (goto _label)))
    (:then_2
      ;[1 1 1] x+2,y+1
      (Variables|Default|SetTempNextYIndex (Math|Float|Floor (Variables|Default|GetYvalue)))
      (Variables|Default|SetTempNextXIndex (Math|Float|Floor (Variables|Default|GetXvalue)))
      (if (and (<= (Variables|Default|GetTempNextXIndex) 7) (>= (Variables|Default|GetTempNextXIndex) 0))
        (bind _output_get_4 (Variables|Default|SetTempNextXIndex (+ (Variables|Default|GetTempNextXIndex) 2)))
        (bind _output_get_5 (Variables|Default|SetTempNextYIndex (+ (Variables|Default|GetTempNextYIndex) 1)))
        (Utilities|Array|Add (Variables|Default|GetVecto2D) (Math|Vector2D|MakeVector2D (* (Math|Conversions|ToFloat(Integer) _output_get_4) 4e+02) (* (Math|Conversions|ToFloat(Integer) _output_get_5) 4e+02)))
        (goto _label)))
    (:then_3
      ;[1 1 1] x+1, y + 2
      (Variables|Default|SetTempNextYIndex (Math|Float|Floor (Variables|Default|GetYvalue)))
      (Variables|Default|SetTempNextXIndex (Math|Float|Floor (Variables|Default|GetXvalue)))
      (if (and (<= (Variables|Default|GetTempNextXIndex) 7) (>= (Variables|Default|GetTempNextXIndex) 0))
        (bind _result_2 (Math|Integer|IncrementInt (Variables|Default|GetTempNextXIndex))
          (:%20%20
            (bind _output_get_6 (Variables|Default|SetTempNextYIndex (+ (Variables|Default|GetTempNextYIndex) 2)))
            (Utilities|Array|Add (Variables|Default|GetVecto2D) (Math|Vector2D|MakeVector2D (* (Math|Conversions|ToFloat(Integer) _result_2) 4e+02) (* (Math|Conversions|ToFloat(Integer) _output_get_6) 4e+02)))
            (goto _label)))))
    (:then_4
      ;[1 1 1] x-1,y+2
      (Variables|Default|SetTempNextYIndex (Math|Float|Floor (Variables|Default|GetYvalue)))
      (Variables|Default|SetTempNextXIndex (Math|Float|Floor (Variables|Default|GetXvalue)))
      (if (and (<= (Variables|Default|GetTempNextXIndex) 7) (>= (Variables|Default|GetTempNextXIndex) 0))
        (bind _result_3 (Math|Integer|DecrementInt (Variables|Default|GetTempNextXIndex))
          (:%20%20
            (bind _output_get_7 (Variables|Default|SetTempNextYIndex (+ (Variables|Default|GetTempNextYIndex) 2)))
            (Utilities|Array|Add (Variables|Default|GetVecto2D) (Math|Vector2D|MakeVector2D (* (Math|Conversions|ToFloat(Integer) _result_3) 4e+02) (* (Math|Conversions|ToFloat(Integer) _output_get_7) 4e+02)))
            (goto _label)))))
    (:then_5
      ;[1 1 1] X-2,y+1
      (Variables|Default|SetTempNextYIndex (Math|Float|Floor (Variables|Default|GetYvalue)))
      (Variables|Default|SetTempNextXIndex (Math|Float|Floor (Variables|Default|GetXvalue)))
      (if (and (<= (Variables|Default|GetTempNextXIndex) 7) (>= (Variables|Default|GetTempNextXIndex) 0))
        (bind _output_get_8 (Variables|Default|SetTempNextXIndex (- (Variables|Default|GetTempNextXIndex) 2)))
        (bind _output_get_9 (Variables|Default|SetTempNextYIndex (+ (Variables|Default|GetTempNextYIndex) 1)))
        (Utilities|Array|Add (Variables|Default|GetVecto2D) (Math|Vector2D|MakeVector2D (* (Math|Conversions|ToFloat(Integer) _output_get_8) 4e+02) (* (Math|Conversions|ToFloat(Integer) _output_get_9) 4e+02)))
        (goto _label)))
    (:then_6
      ;[1 1 1] X-2,y-1
      (Variables|Default|SetTempNextYIndex (Math|Float|Floor (Variables|Default|GetYvalue)))
      (Variables|Default|SetTempNextXIndex (Math|Float|Floor (Variables|Default|GetXvalue)))
      (if (and (<= (Variables|Default|GetTempNextXIndex) 7) (>= (Variables|Default|GetTempNextXIndex) 0))
        (bind _output_get_10 (Variables|Default|SetTempNextXIndex (- (Variables|Default|GetTempNextXIndex) 2)))
        (bind _output_get_11 (Variables|Default|SetTempNextYIndex (- (Variables|Default|GetTempNextYIndex) 1)))
        (Utilities|Array|Add (Variables|Default|GetVecto2D) (Math|Vector2D|MakeVector2D (* (Math|Conversions|ToFloat(Integer) _output_get_10) 4e+02) (* (Math|Conversions|ToFloat(Integer) _output_get_11) 4e+02)))
        (goto _label)))
    (:then_7
      ;[1 1 1] x-1,y-2
      (Variables|Default|SetTempNextYIndex (Math|Float|Floor (Variables|Default|GetYvalue)))
      (Variables|Default|SetTempNextXIndex (Math|Float|Floor (Variables|Default|GetXvalue)))
      (if (and (<= (Variables|Default|GetTempNextXIndex) 7) (>= (Variables|Default|GetTempNextXIndex) 0))
        (bind _output_get_12 (Variables|Default|SetTempNextXIndex (- (Variables|Default|GetTempNextXIndex) 1)))
        (bind _output_get_13 (Variables|Default|SetTempNextYIndex (- (Variables|Default|GetTempNextYIndex) 2)))
        (Utilities|Array|Add (Variables|Default|GetVecto2D) (Math|Vector2D|MakeVector2D (* (Math|Conversions|ToFloat(Integer) _output_get_12) 4e+02) (* (Math|Conversions|ToFloat(Integer) _output_get_13) 4e+02)))
        (goto _label)))))

(fn ConstructionScript
  (|CallParentFunction))