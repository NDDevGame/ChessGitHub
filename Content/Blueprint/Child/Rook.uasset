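; Rook chess piece Blueprint that finds its possible moves and shows them on the chess board.
; Move converts its location to grid coordinates, then steps along X and Y in both directions on a 400-unit grid.
; CheckForValidity line-traces to each candidate square, storing it if unblocked or held by an opposing piece, and the board displays the list.
; Several older move and occupancy-check chains are left disconnected, and RookMovement is empty.
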(event EventBeginPlay
  (|CallParentFunction)
  (Variables|Default|SetID (Variables|Default|GetRookName)))

(event Collision|EventActorBeginOverlap
  (params (OtherActor :type Actor%20Object%20Reference))
  (|CallParentFunction OtherActor) ; This node is disabled and will not be called.\nDrag off pins to build functionality.
)

(event EventTick
  (params (DeltaSeconds :type Float%20%28single-precision%29))
  (|CallParentFunction DeltaSeconds) ; This node is disabled and will not be called.\nDrag off pins to build functionality.
)

(event EventMove
  (params (Location :type Vector :default "0, 0, 0") (ChessBoard :type Chess%20Board%20Object%20Reference))
  (Utilities|Array|Clear (Variables|Default|GetVecto2D))
  (CallFunction|SetPositiontoXYValue Location)
  (Utilities|FlowControl|Sequence
    (:then_0
      ;[1 1 1] Move forward and right
      (Variables|Default|SetTempNextXIndex (Math|Float|Floor (Variables|Default|GetXvalue)))
      (Utilities|FlowControl|ForLoopwithBreak 0 7 :!label _label
        (:LoopBody
          (if (and (<= (Variables|Default|GetTempNextXIndex) 7) (>= (Variables|Default|GetTempNextXIndex) 0))
            (bind _output_get (Variables|Default|SetTempNextXIndex (+ (Variables|Default|GetTempNextXIndex) 1)))
            (Utilities|CheckforValidity (Math|Vector2D|MakeVector2D (* (Math|Conversions|ToFloat(Integer) _output_get) 4e+02) (* (Variables|Default|GetYvalue) 4e+02)))
            (goto _label Break)))
        (:Completed
          (Variables|Default|SetTempNextXIndex 0)
          (Variables|Default|SetTempNextYIndex (Math|Float|Floor (Variables|Default|GetYvalue)))
          (Utilities|FlowControl|ForLoopwithBreak 0 7 :!label _label_2
            (:LoopBody
              (if (and (>= (Variables|Default|GetTempNextYIndex) 0) (<= (Variables|Default|GetTempNextYIndex) 7))
                (Math|Integer|IncrementInt (Variables|Default|GetTempNextYIndex)
                  (:%20%20
                    (Utilities|CheckforValidity (Math|Vector2D|MakeVector2D (* (Variables|Default|GetXvalue) 4e+02) (* (Math|Conversions|ToFloat(Integer) (Variables|Default|GetTempNextYIndex)) 4e+02)))
                    (goto _label_2 Break)))))
            (:Completed
              (Variables|Default|SetTempNextYIndex 0 :!label _label_3)
              (Default|ShowWayMove ChessBoard (Variables|Default|GetVecto2D)))))))
    (:then_1
      ;[1 1 1] Move Backworad and left
      (Variables|Default|SetTempNextXIndex (Math|Float|Floor (Variables|Default|GetXvalue)))
      (Utilities|FlowControl|ForLoopwithBreak 0 7 :!label _label_4
        (:LoopBody
          (if (and (<= (Variables|Default|GetTempNextXIndex) 7) (>= (Variables|Default|GetTempNextXIndex) 0))
            (bind _output_get_2 (Variables|Default|SetTempNextXIndex (- (Variables|Default|GetTempNextXIndex) 1)))
            (Utilities|CheckforValidity (Math|Vector2D|MakeVector2D (* (Math|Conversions|ToFloat(Integer) _output_get_2) 4e+02) (* (Variables|Default|GetYvalue) 4e+02)))
            (goto _label_4 Break)))
        (:Completed
          (Variables|Default|SetTempNextXIndex 0)
          (Variables|Default|SetTempNextYIndex (Math|Float|Floor (Variables|Default|GetYvalue)))
          (Utilities|FlowControl|ForLoopwithBreak 0 7 :!label _label_5
            (:LoopBody
              (if (and (>= (Variables|Default|GetTempNextYIndex) 0) (<= (Variables|Default|GetTempNextYIndex) 7))
                (Math|Integer|DecrementInt (Variables|Default|GetTempNextYIndex)
                  (:%20%20
                    (Utilities|CheckforValidity (Math|Vector2D|MakeVector2D (* (Variables|Default|GetXvalue) 4e+02) (* (Math|Conversions|ToFloat(Integer) (Variables|Default|GetTempNextYIndex)) 4e+02)))
                    (goto _label_5 Break)))))
            (:Completed
              (goto _label_3))))))))

(fn ConstructionScript
  (|CallParentFunction))

(fn RookMovement
  (params (Index :type Integer)))