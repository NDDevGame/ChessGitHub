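; Player controller for a chess game that turns mouse clicks into board selections.
; On BeginPlay it shows the cursor and caches the first Chess_Board actor found in the level.
; On left click it traces under the cursor on the Visibility channel and passes the hit location and actor to the board's OnClickedChessBoard, which receives all click handling.
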(event EventBeginPlay
  (Variables|Default|SetbShowMouseCursor true)
  (bind _outactors (Actor|GetAllActorsOfClass "/Game/Blueprint/chess_Board.chess_Board_C"))
  (bind _aschess_board (Utilities|Casting|CastTochess_Board (Utilities|Array|Get(acopy) _outactors)))
  (bind _output_get (Variables|Default|SetchessBoard_C _aschess_board)))

(event EventTick
  (params (DeltaSeconds :type Float%20%28single-precision%29)))

(event Input|MouseEvents|LeftMouseButton
  (params (Key :type Key%20Structure :default "None"))
  (bind _hitresult (Game|Player|GetHitResultUnderCursorbyChannel "TraceTypeQuery1" true))
  (bind (_bblockinghit _binitialoverlap _time _distance _location _impactpoint _normal _impactnormal _physmat _hitactor) (Collision|BreakHitResult _hitresult))
  (:Pressed
    (Variables|Default|SetLocation _location)
    (Default|OnClickedChessBoard (stale EventBeginPlay _output_get) (Variables|Default|GetLocation) _hitactor)))

(fn ConstructionScript)