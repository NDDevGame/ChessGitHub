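; Chess board actor that builds a 64-tile checkered board in the Construction Script and spawns chess pieces from StartFigures on BeginPlay, sorted into white and black arrays.
; Position helpers convert between tile indices and locations on a 400-unit grid.
; A first click calls the piece's Move, and ShowWayMove highlights given tiles.
; The highlight material doubles as the legality check: a second click there teleports the piece, and any second click clears highlights.
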(event EventBeginPlay
  (bind _chesspieces (Variables|Default|GetChessPieces))
  (for _index (range 0 63)
    (if (Utilities|IsValidClass (Utilities|Select :Index (Utilities|Array|Get(acopy) (Variables|Default|GetStartFigures) _index) :Option%200 0 :Option%201 "/Game/Blueprint/Child/Pawn.Pawn_C" :Option%202 "/Game/Blueprint/Child/Rook.Rook_C" :Option%203 "/Game/Blueprint/Child/Knight.Knight_C" :Option%204 "/Game/Blueprint/Child/Bishop.Bishop_C" :Option%205 "/Game/Blueprint/Child/Queen.Queen_C" :Option%206 "/Game/Blueprint/Child/King.King_C"))
      (bind _returnvalue (Game|SpawnActorfromClass (Utilities|Select :Index (Utilities|Array|Get(acopy) (Variables|Default|GetStartFigures) _index) :Option%200 0 :Option%201 "/Game/Blueprint/Child/Pawn.Pawn_C" :Option%202 "/Game/Blueprint/Child/Rook.Rook_C" :Option%203 "/Game/Blueprint/Child/Knight.Knight_C" :Option%204 "/Game/Blueprint/Child/Bishop.Bishop_C" :Option%205 "/Game/Blueprint/Child/Queen.Queen_C" :Option%206 "/Game/Blueprint/Child/King.King_C") (Math|Transform|MakeTransform (Math|Conversions|ToVector(Vector2D) (+ (.ReturnValue (Utilities|PositionLevelUp _index)) (Math|Conversions|ToVector2D(Vector) (Transformation|GetActorLocation)))) "0, 0, 0" "1,1,1") "Undefined" 0 0))
      (bind _aschess_pieces (Utilities|Casting|CastTochessPieces _returnvalue))
      (Utilities|Array|Add _chesspieces _aschess_pieces)
      (if (> _index 20)
        (Utilities|Array|Add (Variables|Default|GetBlackPieces) _aschess_pieces)
        (else
          (Utilities|Array|Add (Variables|Default|GetWhitePieces) _aschess_pieces)))
      (Default|ConstructPieceData _aschess_pieces (> _index 20))
      (Development|PrintString (Utilities|String|ToString(Integer) (Utilities|Array|Length _chesspieces))))))

(event Collision|EventActorBeginOverlap
  (params (OtherActor :type Actor%20Object%20Reference)))

(event EventTick
  (params (DeltaSeconds :type Float%20%28single-precision%29)))

(fn ConstructionScript
  (for _index (range 0 63)
    (Variables|Default|SetXvalue (* (/ _index 8) 4e+02))
    (Variables|Default|SetYValue (* (Math|Integer|%(Integer) _index 8) 4e+02))
    (bind _returnvalue (AddComponent|AddStaticMeshComponent false (Math|Transform|MakeTransform (Math|Conversions|ToVector(Vector2D) (Math|Vector2D|MakeVector2D (* (/ _index 8) 4e+02) (* (Math|Integer|%(Integer) _index 8) 4e+02))) "0, 0, 0" "1,1,1")))
    (Utilities|Array|Add (Variables|Default|GetChessBoard) (Math|Vector2D|MakeVector2D (* (/ _index 8) 4e+02) (* (Math|Integer|%(Integer) _index 8) 4e+02)))
    (Utilities|Array|Add (Variables|Default|GetChessBoard_Mesh%20) _returnvalue)
    (Rendering|Material|SetMaterial _returnvalue 0 (select (Class|KismetMathLibrary|XORBoolean (Math|Conversions|ToBoolean(Integer) (Math|Integer|%(Integer) _index 2)) (Math|Conversions|ToBoolean(Integer) (Math|Integer|%(Integer) (/ _index 8) 2))) "/Game/Material/M_Black.M_Black" "/Game/Material/M_White.M_White"))
    (Utilities|Array|Add (Variables|Default|GetChessBoard_Material) (select (Class|KismetMathLibrary|XORBoolean (Math|Conversions|ToBoolean(Integer) (Math|Integer|%(Integer) _index 2)) (Math|Conversions|ToBoolean(Integer) (Math|Integer|%(Integer) (/ _index 8) 2))) "/Game/Material/M_Black.M_Black" "/Game/Material/M_White.M_White"))))

(fn ChessBoardonClickedtoIndex
  (params (Position :type Vector))
  (return (Utilities|Position->Index Position)))

(fn ShowWayMove
  (params (Vecto2D :type Array%20of%20Vector%202D%20Structures))
  (bind _chessboard (Variables|Default|GetChessBoard))
  (for _array_element Vecto2D
    (if (Utilities|Array|ContainsItem _chessboard _array_element)
      (Rendering|Material|SetMaterial (Utilities|Array|Get(acopy) (Variables|Default|GetChessBoard_Mesh%20) (Utilities|Array|FindItem _chessboard _array_element)) 0 "/Game/Material/M_OnClicked.M_OnClicked"))))

(fn CheckforValidityBlackPieces
  (params (NextMove :type Vector%202D%20Structure))
  (for _array_element (Variables|Default|GetBlackPieces)
    _)
  (return (Math|Vector|Equal(Vector) NextMove (Math|Vector2D|MakeVector2D (/ (.X (Math|Vector|BreakVector (Transformation|GetActorLocation _array_element))) 4e+02) (/ (.Y (Math|Vector|BreakVector (Transformation|GetActorLocation _array_element))) 4e+02)) 0.0001)))

(fn OnClickedChessBoard
  (params (InLocation :type Vector) (Actor :type Actor%20Object%20Reference))
  (bind _returnvalue (Utilities|Position->Index InLocation))
  (if (== (Variables|Default|GetLastclick) -1)
    (Variables|Default|SetLastclick _returnvalue)
    (bind _aschess_pieces (Utilities|Casting|CastTochessPieces Actor))
    (Default|Move _aschess_pieces InLocation self)
    (bind _output_get (Variables|Default|SetIndex (Utilities|Array|FindItem (Variables|Default|GetChessPieces) _aschess_pieces)))
    (else
      (Development|PrintString "false")
      (if (== (Rendering|Material|GetMaterial (Utilities|Array|Get(acopy) (Variables|Default|GetChessBoard_Mesh%20) _returnvalue) 0) "/Game/Material/M_OnClicked.M_OnClicked")
        (Development|PrintString "Hello")
        (for (_array_element _array_index) (Variables|Default|GetChessBoard_Mesh%20)
          (Rendering|Material|SetMaterial _array_element 0 (Utilities|Array|Get(acopy) (Variables|Default|GetChessBoard_Material) _array_index)))
        (Transformation|SetWorldLocation (Variables|/Game/Blueprint/chessPieces.chessPieces_C|GetDefaultSceneRoot (Utilities|Array|Get(acopy) (Variables|Default|GetChessPieces) _output_get)) (.Position+200 (Utilities|PositionLevelUp _returnvalue)) false true)
        (Actor|GetAllActorsOfClass 0)
        (Variables|Default|SetLastclick -1)
        (else
          (for (_array_element_2 _array_index_2) (Variables|Default|GetChessBoard_Mesh%20)
            (Rendering|Material|SetMaterial _array_element_2 0 (Utilities|Array|Get(acopy) (Variables|Default|GetChessBoard_Material) _array_index_2)))
          (Variables|Default|SetLastclick -1))))))