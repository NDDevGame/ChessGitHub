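; Chess piece actor, apparently a base for pieces, that stores its side and its square on the board.
; The construction script and ConstructPieceData set the mesh to a black or white material from the Side boolean.
; SetPositiontoXYValue floors a position onto a 400-unit grid, and helper graphs hold the math from index or X/Y back to position.
; The Move event takes a location and chessboard but has no logic here.
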(event Custom|Move
  (params (Location :type Vector) (ChessBoard :type Chess%20Board%20Object%20Reference)))

(event EventBeginPlay)

(event Collision|EventActorBeginOverlap
  (params (OtherActor :type Actor%20Object%20Reference)))

(event EventTick
  (params (DeltaSeconds :type Float%20%28single-precision%29)))

(fn ConstructionScript
  (Rendering|Material|SetMaterial (Variables|Default|GetChessMesh) 0 (select (Variables|Default|GetSide) "/Game/Material/M_BlackChess.M_BlackChess" "/Game/Material/M_WhiteChess.M_WhiteChess")))

(fn ConstructPieceData
  (params (Side :type Boolean))
  (Variables|Default|SetSide Side)
  (Rendering|Material|SetMaterial (Variables|Default|GetChessMesh) 0 (select (Variables|Default|GetSide) "/Game/Material/M_BlackChess.M_BlackChess" "/Game/Material/M_WhiteChess.M_WhiteChess")))

(fn SetPositiontoXYValue
  (params (Position :type Vector))
  (bind _returnvalue (/ Position "400.000000,400.000000,1.000000"))
  (bind (_x _y) (Math|Vector|BreakVector _returnvalue))
  (Variables|Default|SetXvalue (Math|Conversions|ToFloat(Integer) (Math|Float|Floor _x)))
  (Variables|Default|SetYvalue (Math|Conversions|ToFloat(Integer) (Math|Float|Floor _y))))